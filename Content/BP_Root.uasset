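; BP_Root is an actor that grows a randomized, tapering root from spline meshes, with its length driven by Score.
; BeginPlay rebuilds the spline along negative X with random Y-free jitter in X and Z, using Score divided by Test for point count.
; RefreshMesh tiles non-colliding meshes by SectionLength, clamping tangents and shrinking cross-section toward the tip.
; The construction script builds untapered segments along the existing spline.
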(event Custom|RefreshMesh
  (bind _spline (Variables|Default|GetSpline))
  (bind _spline_2 (Variables|Default|GetSpline))
  (bind _returnvalue (Spline|GetSplineLength _spline))
  (bind _returnvalue_2 (Spline|GetSplineLength _spline_2))
  (if (Variables|Default|GetAllowScaling)
    (bind _output_get (Variables|Default|SetSectionLength (* (.z (Transformation|GetActorScale3D)) 1e+02)))
    (Development|PrintString (Utilities|String|ToString(Float) _output_get)))
  (for _index (range 0 (- (Math|Float|Truncate (/ (Spline|GetSplineLength (Variables|Default|GetSpline)) (Variables|Default|GetSectionLength))) 1))
    (Variables|Default|SetIndex _index)
    (bind _returnvalue_3 (AddComponent|AddSplineMeshComponent false))
    (Components|StaticMesh|SetStaticMesh _returnvalue_3 (Variables|Default|GetNew%20Mesh))
    (SplineMesh|SetForwardAxis _returnvalue_3 "Z" true)
    (bind (_position _tan) (CallFunction|GetStartPositionandTan (Variables|Default|GetIndex)))
    (bind (_position_2 _tan_2) (CallFunction|GetEndPositionandTan (Variables|Default|GetIndex)))
    (SplineMesh|SetStartandEnd _returnvalue_3 _position _tan _position_2 _tan_2 true :!class /Script/Engine.SplineMeshComponent)
    (Collision|SetCollisionEnabled _returnvalue_3 "NoCollision")
    (SplineMesh|SetStartScale _returnvalue_3 (Math|Vector2D|MakeVector2D (/ (- _returnvalue_2 (* (Variables|Default|GetIndex) (Variables|Default|GetSectionLength))) _returnvalue_2) (/ (- _returnvalue_2 (* (Variables|Default|GetIndex) (Variables|Default|GetSectionLength))) _returnvalue_2)) true :!class /Script/Engine.SplineMeshComponent)
    (SplineMesh|SetEndScale _returnvalue_3 (Math|Vector2D|MakeVector2D (/ (- _returnvalue (* (+ (Variables|Default|GetIndex) 1) (Variables|Default|GetSectionLength))) _returnvalue) (/ (- _returnvalue (* (+ (Variables|Default|GetIndex) 1) (Variables|Default|GetSectionLength))) _returnvalue)) true :!class /Script/Engine.SplineMeshComponent)))

(event EventBeginPlay
  (bind _spline (Variables|Default|GetSpline))
  (bind _spline_2 (Variables|Default|GetSpline))
  (Spline|ClearSplinePoints _spline_2 true)
  (Class|SplineComponent|AddPoint _spline_2 (Utilities|Struct|MakeSplinePoint 0.0 "0.000000,0.000000,0.000000" "0.000000,0.000000,0.000000" "0.000000,0.000000,-0.000000" "0.000000,0.000000,0.000000" "1.000000,1.000000,1.000000" "Curve") true)
  (Class|SplineComponent|AddPoint _spline_2 (Utilities|Struct|MakeSplinePoint 1.0 "-100.000000,0.000000,0.000000" "0.000000,0.000000,0.000000" "0.000000,0.000000,-0.000000" "0.000000,0.000000,0.000000" "1.000000,1.000000,1.000000" "Curve") true)
  (for _index (range 2 (Math|Float|Ceil (/ (Variables|Default|GetScore) (Variables|Default|GetTest))))
    (Class|SplineComponent|AddPoint _spline (Utilities|Struct|MakeSplinePoint (Math|Conversions|ToFloat(Integer) _index) (Math|Vector|MakeVector (+ (Math|Conversions|ToFloat(Integer) (* _index -100)) (select (<= _index 0) 0.0 (Math|Random|RandomFloatinRange -25.0 25.0))) 0.0 (Math|Random|RandomFloatinRange -2e+02 2e+02))) true))
  (Development|PrintString (Utilities|String|ToString(Integer) (Spline|GetNumberOfSplinePoints _spline)))
  (CallFunction|RefreshMesh))

(fn ConstructionScript
  (if (Variables|Default|GetAllowScaling)
    _
    (else
      _))
  (bind _output_get (Variables|Default|SetSectionLength (* (.z (Transformation|GetActorScale3D)) 1e+02)))
  (Development|PrintString (Utilities|String|ToString(Float) _output_get))
  (for _index (range 0 (- (Math|Float|Truncate (/ (Spline|GetSplineLength (Variables|Default|GetSpline)) (Variables|Default|GetSectionLength))) 1))
    (Variables|Default|SetIndex _index)
    (bind _returnvalue (AddComponent|AddSplineMeshComponent false))
    (Components|StaticMesh|SetStaticMesh _returnvalue (Variables|Default|GetNew%20Mesh))
    (SplineMesh|SetForwardAxis _returnvalue "Z" true)
    (bind (_position _tan) (CallFunction|GetStartPositionandTan (Variables|Default|GetIndex)))
    (bind (_position_2 _tan_2) (CallFunction|GetEndPositionandTan (Variables|Default|GetIndex)))
    (SplineMesh|SetStartandEnd _returnvalue _position _tan _position_2 _tan_2 true :!class /Script/Engine.SplineMeshComponent)
    (Collision|SetCollisionEnabled _returnvalue "NoCollision")))

(fn GetEndPositionandTan
  (params (Index :type Integer))
  (bind _returnvalue (+ Index 1))
  (bind _sectionlength (Variables|Default|GetSectionLength))
  (bind _returnvalue_2 (* _returnvalue _sectionlength))
  (return (Spline|GetLocationatDistanceAlongSpline (Variables|Default|GetSpline) _returnvalue_2 "Local") (Math|Vector|ClampVectorSize (Spline|GetTangentatDistanceAlongSpline (Variables|Default|GetSpline) _returnvalue_2 "Local") 0.0 (Variables|Default|GetSectionLength))))

(fn GetStartPositionandTan
  (params (Index :type Integer))
  (bind _sectionlength (Variables|Default|GetSectionLength))
  (bind _returnvalue (* Index _sectionlength))
  (return (Spline|GetLocationatDistanceAlongSpline (Variables|Default|GetSpline) _returnvalue "Local") (Math|Vector|ClampVectorSize (Spline|GetTangentatDistanceAlongSpline (Variables|Default|GetSpline) _returnvalue "Local") 0.0 (Variables|Default|GetSectionLength))))