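; BP_Tree is an interactable tree that the player waters to build up a score.
; Interact succeeds only if the character has water, in which case it consumes that water and calls Arroser.
; Arroser starts a fast looping timer that increments and prints Score, plus a one-shot timer that stops it after a few seconds.
; AbortInteraction also clears the looping timer, ending watering early.
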(event Custom|Arroser
  (bind _returnvalue (Utilities|Time|SetTimerbyEvent (delegate Custom|CustomEvent) 0.01 true))
  (Variables|Default|SetTimerArrosoir _returnvalue)
  (Utilities|Time|SetTimerbyEvent (delegate Custom|CustomEvent_0) 5.0))

(event Custom|CustomEvent
  (bind _output_get (Variables|Default|Setscore (+ (Variables|Default|Getscore) 1.0)))
  (Development|PrintString (Utilities|String|ToString(Float) _output_get) true true "(R=1.000000,G=0.000000,B=0.810636,A=1.000000)" 1.0))

(event Custom|CustomEvent_0
  (Utilities|Time|ClearandInvalidateTimerbyHandle (Variables|Default|GetTimerArrosoir)))

(event EventAbortInteraction
  (Utilities|Time|ClearandInvalidateTimerbyHandle (Variables|Default|GetTimerArrosoir)))

(fn ConstructionScript)

(fn Interact
  (params (Chara :type BP%20Character%20Object%20Reference))
  (if (Variables|/Game/Blueprints/Character/BP_Character.BP_Character_C|GetHasWater Chara)
    (CallFunction|Arroser)
    (Variables|/Game/Blueprints/Character/BP_Character.BP_Character_C|SetHasWater Chara false)
    (return true)
    (else
      (return false))))