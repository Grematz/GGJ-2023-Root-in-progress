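; BPC_CharacterTheo is a character Blueprint that runs a minute, second and millisecond countdown and shows a timer widget.
; BeginPlay creates WBP_Timer, adds it to the viewport and starts a looping 0.01-second timer event.
; Each call decrements Miliseconds, which wraps at 59 into Seconds and then Minutes, so it runs faster than real time.
; Minutes reaching zero only prints a debug string; the timer keeps looping.
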(event Custom|Timer
  (bind _result (Math|Integer|DecrementInt (Variables|Default|GetMiliseconds))
    (:%20%20
      (if (== _result -1)
        (Variables|Default|SetMiliseconds 59)
        (bind _result_2 (Math|Integer|DecrementInt (Variables|Default|GetSeconds))
          (:%20%20
            (if (== _result_2 -1)
              (Variables|Default|SetSeconds 59)
              (bind _result_3 (Math|Integer|DecrementInt (Variables|Default|GetMinutes))
                (:%20%20
                  (if (== _result_3 0)
                    (Development|PrintString "Hello")))))))))))

(event EventBeginPlay
  (|CallParentFunction)
  (bind _returnvalue (UserInterface|CreateWidget "/Game/UI/WBP_Timer.WBP_Timer_C"))
  (UserInterface|Viewport|AddtoViewport _returnvalue 0)
  (Utilities|Time|SetTimerbyEvent (delegate Custom|Timer) 0.01 true))

(event Collision|EventActorBeginOverlap
  (params (OtherActor :type Actor%20Object%20Reference))
  (|CallParentFunction OtherActor) ; This node is disabled and will not be called.\nDrag off pins to build functionality.
)

(event EventTick
  (params (DeltaSeconds :type Float%20%28single-precision%29))
  (|CallParentFunction DeltaSeconds) ; This node is disabled and will not be called.\nDrag off pins to build functionality.
)

(fn ConstructionScript
  (|CallParentFunction))