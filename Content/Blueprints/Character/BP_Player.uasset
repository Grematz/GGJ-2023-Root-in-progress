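; BP_Player is the player Blueprint that provides click-to-move control of a separate ControlledCharacter.
; On IA_Interact, it runs a debug-drawn Visibility line trace from the camera location using the deprojected mouse direction.
; If the hit actor lacks BPI_Interact, AIMoveTo sends the character to the hit location.
; Hits on interactable actors currently trigger nothing.
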(event Input|EnhancedActionEvents|EnhancedInputActionIA_Interact
  (params (ActionValue :type Boolean) (ElapsedSeconds :type Float%20%28double-precision%29) (TriggeredSeconds :type Float%20%28double-precision%29) (InputAction :type Input%20Action%20Object%20Reference :default "/Game/Blueprints/Inputs/Actions/IA_Interact.IA_Interact"))
  (:Started
    (bind _outhit (Collision|LineTraceByChannel (Camera|GetCameraLocation (Game|GetPlayerCameraManager 0)) (* (.WorldDirection (Game|Player|ConvertMouseLocationToWorldSpace (Game|GetPlayerController 0))) 1000000000) "TraceTypeQuery1" false 0 "ForDuration"))
    (if (not (Utilities|DoesObjectImplementInterface (.HitActor (Collision|BreakHitResult _outhit)) "/Game/Blueprints/BPI_Interact.BPI_Interact_C"))
      (AI|AIMoveTo (Variables|Default|GetControlledCharacter) (.Location (Collision|BreakHitResult _outhit)) 0 5.0 false))))

(event EventBeginPlay)

(event Collision|EventActorBeginOverlap
  (params (OtherActor :type Actor%20Object%20Reference)))

(event EventTick
  (params (DeltaSeconds :type Float%20%28single-precision%29)))

(fn ConstructionScript)