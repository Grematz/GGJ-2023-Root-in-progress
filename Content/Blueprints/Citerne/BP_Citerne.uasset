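; Interactable water tank that gives a bucket of water to a character who has none, then goes on cooldown.
; Interact succeeds only when the tank is usable, calling HoldBucket on the character and starting the cooldown.
; A fast looping timer advances CoolDown at half real-time rate until CoolDownMax re-enables the tank.
; On BeginPlay it passes itself to the WBP_WaterTankCD widget in its UICD component.
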(event Custom|CDTimer
  (bind _output_get (Variables|Default|SetCoolDown (+ (Variables|Default|GetCoolDown) 0.005)))
  (if (>= _output_get (Variables|Default|GetCoolDownMax))
    (Variables|Default|SetCanUsed true)
    (Utilities|Time|ClearandInvalidateTimerbyHandle (Variables|Default|GetTimerBreak))))

(event Custom|Start%20Cooldown
  (Variables|Default|SetCoolDown 0.0)
  (Variables|Default|SetCanUsed false)
  (bind _returnvalue (Utilities|Time|SetTimerbyEvent (delegate Custom|CDTimer) 0.01 true))
  (Variables|Default|SetTimerBreak _returnvalue))

(event EventBeginPlay
  (bind _aswbp_water_tank_cd (Utilities|Casting|CastToWBP_WaterTankCD (UserInterface|GetWidget (Variables|Default|GetUI_CD))))
  (Variables|/Game/UI/WBP_WaterTankCD.WBP_WaterTankCD_C|SetWaterTankRef _aswbp_water_tank_cd self))

(event Collision|EventActorBeginOverlap
  (params (OtherActor :type Actor%20Object%20Reference)))

(event EventTick
  (params (DeltaSeconds :type Float%20%28single-precision%29)))

(fn ConstructionScript)

(fn Interact
  (params (Chara :type BP%20Character%20Object%20Reference))
  (if (and (Variables|Default|GetCanUsed) (not (Variables|/Game/Blueprints/Character/BP_Character.BP_Character_C|GetHasWater Chara)))
    (Default|HoldBucket Chara)
    (CallFunction|StartCooldown)
    (return true)
    (else
      (return false))))