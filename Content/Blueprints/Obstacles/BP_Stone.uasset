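; BP_Stone is an interactable obstacle that a character mines away over a short hold of progress.
; Interact plays the Pull_Plant montage on the character and calls Mine, which shows a progress widget component and starts a looping timer.
; Each timer tick raises Percent until it is full and the stone destroys itself.
; AbortInteraction clears the timer, resets Percent and hides the widget.
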(event Custom|Mine
  (bind _returnvalue (Utilities|Time|SetTimerbyEvent (delegate Custom|MiningEvent) 0.01 true))
  (Variables|Default|SetMiningTimer _returnvalue)
  (Rendering|SetVisibility (Variables|Default|GetWidget) true false))

(event Custom|MiningEvent
  (bind _output_get (Variables|Default|SetPercent (+ (Variables|Default|GetPercent) 0.005)))
  (if (>= _output_get 1.0)
    (Actor|DestroyActor)))

(event Collision|EventActorBeginOverlap
  (params (OtherActor :type Actor%20Object%20Reference))
  (|CallParentFunction OtherActor) ; This node is disabled and will not be called.\nDrag off pins to build functionality.
)

(event EventTick
  (params (DeltaSeconds :type Float%20%28single-precision%29))
  (|CallParentFunction DeltaSeconds) ; This node is disabled and will not be called.\nDrag off pins to build functionality.
)

(event EventBeginPlay
  (bind _returnvalue (UserInterface|CreateWidget "/Game/UI/WBP_TaskProgressionObstacles.WBP_TaskProgressionObstacles_C" 0 self))
  (UserInterface|SetWidget (Variables|Default|GetWidget) _returnvalue))

(event EventAbortInteraction
  (Utilities|Time|ClearandInvalidateTimerbyHandle (Variables|Default|GetMiningTimer))
  (Variables|Default|SetPercent 0.0)
  (Rendering|SetVisibility (Variables|Default|GetWidget) false false))

(fn ConstructionScript
  (|CallParentFunction))

(fn Interact
  (params (Chara :type BP%20Character%20Object%20Reference))
  (Animation|PlayAnimMontage Chara "/Game/Character/Pull_Plant_Montage.Pull_Plant_Montage" 2.5 "None")
  (CallFunction|Mine)
  (return true))