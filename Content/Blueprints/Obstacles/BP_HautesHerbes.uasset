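; Tall grass obstacle that slows any BP_Character inside its box and can be cut down through interaction.
; Box overlap begin and end call the character's Slow and RestSlow functions.
; Interact starts a looping timer that raises Percent until the actor destroys itself, while AbortInteraction clears the timer and resets progress.
; A task progression widget is created on BeginPlay and assigned to the widget component.
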(event OnComponentBeginOverlap(Box)
  (params (OverlappedComponent :type Primitive%20Component%20Object%20Reference) (OtherActor :type Actor%20Object%20Reference) (OtherComp :type Primitive%20Component%20Object%20Reference) (OtherBodyIndex :type Integer) (bFromSweep :type Boolean) (SweepResult :type Hit%20Result%20Structure%20%28by%20ref%29))
  (bind _asbp_character (Utilities|Casting|CastToBP_Character OtherActor))
  ;[1 1 1] Slow PlayerSpeed
  (Default|Slow _asbp_character))

(event OnComponentEndOverlap(Box)
  (params (OverlappedComponent :type Primitive%20Component%20Object%20Reference) (OtherActor :type Actor%20Object%20Reference) (OtherComp :type Primitive%20Component%20Object%20Reference) (OtherBodyIndex :type Integer))
  (bind _asbp_character (Utilities|Casting|CastToBP_Character OtherActor))
  ;[1 1 1] Up PlayerSpeed
  (Default|RestSlow _asbp_character))

(event Custom|Couper
  (bind _returnvalue (Utilities|Time|SetTimerbyEvent (delegate Custom|CouperEvent) 0.01 true))
  (Variables|Default|SetCutTimer _returnvalue))

(event Custom|CouperEvent
  (bind _output_get (Variables|Default|SetPercent (+ (Variables|Default|GetPercent) 0.01)))
  (if (>= _output_get 1.0)
    (Actor|DestroyActor)))

(event Collision|EventActorBeginOverlap
  (params (OtherActor :type Actor%20Object%20Reference))
  (|CallParentFunction OtherActor) ; This node is disabled and will not be called.\nDrag off pins to build functionality.
)

(event EventTick
  (params (DeltaSeconds :type Float%20%28single-precision%29))
  (|CallParentFunction DeltaSeconds) ; This node is disabled and will not be called.\nDrag off pins to build functionality.
)

(event EventAbortInteraction
  (Utilities|Time|ClearandInvalidateTimerbyHandle (Variables|Default|GetCutTimer))
  (Variables|Default|SetPercent 0.0))

(event EventBeginPlay
  (bind _returnvalue (UserInterface|CreateWidget "/Game/UI/WBP_TaskProgression.WBP_TaskProgression_C" 0 self))
  (UserInterface|SetWidget (Variables|Default|GetWidget) _returnvalue))

(fn ConstructionScript
  (|CallParentFunction))

(fn Interact
  (params (Chara :type BP%20Character%20Object%20Reference))
  (CallFunction|Couper)
  (return true))